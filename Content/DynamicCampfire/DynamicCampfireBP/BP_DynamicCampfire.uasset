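; Interactable campfire actor that toggles between lit and extinguished with lighter and extinguish sounds, and prompts the demo HUD crosshair.
; Tick ramps temperature, flame scale, loop volume and light up or down by fixed per-frame steps, with random intensity flicker on alternate frames.
; Firelighter burn, branch charring and fish cooking via material and morph target only advance while burning.
; The construction script creates the dynamic materials, applies color tints and toggles optional rocks and fish.
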(event `/Game/DynamicCampfire/FirstPersonCharacter/Input/BPI_Interact.IsInteractable`
  ;[1 1 1] Interaction
  (bind _ashud_dynamic_campire_demo (cast `/Game/DynamicCampfire/FirstPersonCharacter/HUD/HUD_DynamicCampire_Demo` (`PlayerController.GetHUD` (`GameplayStatics.GetPlayerController` 0))))
  (`/Game/DynamicCampfire/FirstPersonCharacter/HUD/HUD_DynamicCampire_Demo.Crosshair Interact` _ashud_dynamic_campire_demo))

(event `/Game/DynamicCampfire/FirstPersonCharacter/Input/BPI_Interact.Interaction`
  ;[1 1 1] Interaction
  (if (`self.Burning`)
    (set `self.Burning` false)
    (`GameplayStatics.PlaySoundAtLocation` "/Game/DynamicCampfire/DynamicCampfireBP/SoundFX/SW_Extinguish.SW_Extinguish" (0.0 0.0 0.0) (struct) 1.0 1.0 0.0 null null null null)
    (else
      (set `self.Burning` true)
      (`GameplayStatics.PlaySoundAtLocation` "/Game/DynamicCampfire/DynamicCampfireBP/SoundFX/SW_Lighter.SW_Lighter" (0.0 0.0 0.0) (struct) 1.0 1.0 0.0 null null null null))))

(event `self.ReceiveTick`
  (params (DeltaSeconds :type "Float (single-precision)"))
  (bind _temperature (`self.Temperature`))
  (bind _flame_attenuation_max (`self.Flame Attenuation Max`))
  (bind _flameslight (`self.FlamesLight`))
  (bind _burning_branches_material (`self.Burning Branches Material`))
  (bind _ashes_material (`self.Ashes Material`))
  (bind _flame_intensity_max (`self.Flame Intensity Max`))
  (bind _flame_intensity (`self.Flame Intensity`))
  (bind _burningloop (`self.BurningLoop`))
  (bind _flame_size_max (`self.Flame Size Max`))
  (bind _firelighter_material (`self.Firelighter Material`))
  (bind _flame_size (`self.Flame Size`))
  (bind _temperature_max (`self.Temperature Max`))
  (bind _flame_intensity_2 (`self.Flame Intensity`))
  (bind _flame_attenuation (`self.Flame Attenuation`))
  (bind _returnvalue (* (`self.Flame Size`) 2.0))
  (`|ExecutionSequence`
    (:`then_0`
      ;[1 0.07149 0] Burning Process
      ;;[1 1 1] Light Random Flickering
      (`/Engine/EditorBlueprintResources/StandardMacros.FlipFlop`
        (:`A`
          (`LightComponent.SetIntensity` (`self.FlamesLight`) (+ _flame_intensity (* (/ _flame_intensity 10.0) (`KismetMathLibrary.RandomFloatInRange` 0.0 5.0)))))))
    (:`then_1`
      (if (`self.Burning`)
        ;;[1 1 1] Firelighter Burn
        (bind _output_get (set `self.Firelighter Burn` (`KismetMathLibrary.FClamp` (- (`self.Firelighter Burn`) 0.0025) -2.5 2.0)))
        (`MaterialInstanceDynamic.SetScalarParameterValue` (`self.Firelighter Material`) "Firelighter" _output_get)
        ;;[1 1 1] Smoked and Burned
        (bind _output_get_2 (set `self.Smoked` (`KismetMathLibrary.FClamp` (+ (`self.Smoked`) 0.0005) 0.0 (`self.Smoked Max`))))
        (`MaterialInstanceDynamic.SetScalarParameterValue` (`self.Burning Branches Material`) "Smoked" _output_get_2)
        (bind _output_get_3 (set `self.Burned` (`KismetMathLibrary.FClamp` (+ (`self.Burned`) 0.0001) 0.0 (`self.Burned Max`))))
        (`MaterialInstanceDynamic.SetScalarParameterValue` (`self.Burning Branches Material`) "Burned" _output_get_3)
        ;;[1 1 1] Temperature
        (bind _output_get_4 (set `self.Temperature` (`KismetMathLibrary.FClamp` (+ _temperature 0.001) 0.0 _temperature_max)))
        (`MaterialInstanceDynamic.SetScalarParameterValue` _burning_branches_material "Temperature" _output_get_4)
        (`MaterialInstanceDynamic.SetScalarParameterValue` _ashes_material "Temperature" _output_get_4)
        (`MaterialInstanceDynamic.SetScalarParameterValue` _firelighter_material "Temperature" _output_get_4)
        ;;[1 1 1] Particles
        (bind _output_get_5 (set `self.Flame Size` (`KismetMathLibrary.FClamp` (+ _flame_size 0.003) 0.0 _flame_size_max)))
        (`SceneComponent.SetRelativeScale3D` (`self.N_CampfireFlames`) (`KismetMathLibrary.MakeVector` _output_get_5 _output_get_5 1.0))
        ;;[1 1 1] Sound
        (`AudioComponent.SetVolumeMultiplier` _burningloop _returnvalue)
        ;;[1 1 1] Light
        (set `self.Flame Intensity` (`KismetMathLibrary.FClamp` (+ _flame_intensity_2 1.5) 0.0 _flame_intensity_max))
        (bind _output_get_6 (set `self.Flame Attenuation` (`KismetMathLibrary.FClamp` (+ _flame_attenuation 1.0) 0.0 _flame_attenuation_max)))
        (`LocalLightComponent.SetAttenuationRadius` _flameslight _output_get_6)
        ;;[0 0.9675 1] Fish Cooking
        (bind _output_get_7 (set `self.Cooked` (`KismetMathLibrary.FClamp` (+ (`self.Cooked`) 0.0001))))
        (`MaterialInstanceDynamic.SetScalarParameterValue` (`self.Cooking Fish Material`) "Cooked" _output_get_7)
        (`SkeletalMeshComponent.SetMorphTarget` (`self.SK_FishCooking`) "Cooked" _output_get_7 true)
        (else
          (bind _output_get_8 (set `self.Temperature` (`KismetMathLibrary.FClamp` (- _temperature 0.001) 0.0 _temperature_max)))
          (`MaterialInstanceDynamic.SetScalarParameterValue` _burning_branches_material "Temperature" _output_get_8)
          (`MaterialInstanceDynamic.SetScalarParameterValue` _ashes_material "Temperature" _output_get_8)
          (`MaterialInstanceDynamic.SetScalarParameterValue` _firelighter_material "Temperature" _output_get_8)
          (bind _output_get_9 (set `self.Flame Size` (`KismetMathLibrary.FClamp` (- _flame_size 0.005) 0.0 _flame_size_max)))
          (`SceneComponent.SetRelativeScale3D` (`self.N_CampfireFlames`) (`KismetMathLibrary.MakeVector` _output_get_9 _output_get_9 1.0))
          (`AudioComponent.SetVolumeMultiplier` _burningloop _returnvalue)
          (set `self.Flame Intensity` (`KismetMathLibrary.FClamp` (- _flame_intensity_2 6.0) 0.0 _flame_intensity_max))
          (bind _output_get_10 (set `self.Flame Attenuation` (`KismetMathLibrary.FClamp` (- _flame_attenuation 4.0) 0.0 _flame_attenuation_max)))
          (`LocalLightComponent.SetAttenuationRadius` _flameslight _output_get_10))))))

(fn `UserConstructionScript`
  (bind _sm_campfirerocks (`self.SM_CampfireRocks`))
  (bind _sk_fishcooking (`self.SK_FishCooking`))
  ;[1 1 1] Create Dynamic Material Instances
  (bind _returnvalue (`DecalComponent.CreateDynamicMaterialInstance` (`self.Ashes Decal`)))
  (set `self.Ashes Material` _returnvalue)
  (bind _returnvalue_2 (`PrimitiveComponent.CreateDynamicMaterialInstance` (`self.SK_FishCooking`) 0 "/Game/DynamicCampfire/DynamicCampfireBP/Materials/M_Fish_Dynamic.M_Fish_Dynamic" "None"))
  (set `self.Cooking Fish Material` _returnvalue_2)
  (bind _returnvalue_3 (`PrimitiveComponent.CreateDynamicMaterialInstance` (`self.SM_CampfireBranches`) 0 "/Game/DynamicCampfire/DynamicCampfireBP/Materials/M_CampfireBranches_Dynamic.M_CampfireBranches_Dynamic" "None"))
  (set `self.Burning Branches Material` _returnvalue_3)
  (bind _returnvalue_4 (`PrimitiveComponent.CreateDynamicMaterialInstance` (`self.SM_CampfireFirelighter`) 0 "/Game/DynamicCampfire/DynamicCampfireBP/Materials/M_CampfireFirelighter_Dynamic.M_CampfireFirelighter_Dynamic" "None"))
  (set `self.Firelighter Material` _returnvalue_4)
  (bind _returnvalue_5 (`PrimitiveComponent.CreateDynamicMaterialInstance` (`self.SM_CampfireRocks`) 0 "/Game/DynamicCampfire/DynamicCampfireBP/Materials/M_CampfireRocks.M_CampfireRocks" "None"))
  (set `self.Rocks Material` _returnvalue_5)
  ;[1 1 1] Color Adjusts
  (`MaterialInstanceDynamic.SetVectorParameterValue` (`self.Burning Branches Material`) "Branches Color Adjust" (`KismetMathLibrary.Conv_ColorToLinearColor` (`self.Branches Color Adjust`)))
  (`MaterialInstanceDynamic.SetVectorParameterValue` (`self.Firelighter Material`) "Firelighter Color Adjust" (`KismetMathLibrary.Conv_ColorToLinearColor` (`self.Firelighter Color Adjust`)))
  (`MaterialInstanceDynamic.SetVectorParameterValue` (`self.Rocks Material`) "Rocks Color Adjust" (`KismetMathLibrary.Conv_ColorToLinearColor` (`self.Rocks Color Adjust`)))
  ;[1 1 1] Sow/Hide Components
  (`|ExecutionSequence`
    (:`then_0`
      (if (`self.Rocks`)
        (`SceneComponent.SetVisibility` _sm_campfirerocks true false)
        (else
          (`SceneComponent.SetVisibility` _sm_campfirerocks false false))))
    (:`then_1`
      (if (`self.Fish`)
        (`SceneComponent.SetVisibility` _sk_fishcooking true false)
        (`SceneComponent.SetVisibility` (`self.SM_FishCookingSticks`) true false)
        (else
          (`SceneComponent.SetVisibility` _sk_fishcooking false false)
          (`SceneComponent.SetVisibility` (`self.SM_FishCookingSticks`) false false))))))