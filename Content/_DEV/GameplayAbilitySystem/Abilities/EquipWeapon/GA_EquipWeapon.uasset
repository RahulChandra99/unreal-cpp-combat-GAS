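; Gameplay ability that equips or unequips the avatar's weapon when triggered by a gameplay event.
; After committing, it switches on the event's first target tag to have the avatar's WeaponsManagerComponent equip the staff, axe or shield, or unequip by default.
; The staff also plays a sound at world origin.
; The ability ends afterwards, but only when that component is valid; otherwise EndAbility is never called.
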(event `self.K2_ActivateAbilityFromEvent`
  (params (EventData :type "GameplayEventData Structure (by ref)"))
  (bind _returnvalue (`Actor.GetComponentByClass` (`self.GetAvatarActorFromActorInfo`) "/Game/_DEV/Weapons/WeaponsManagerComponent.WeaponsManagerComponent_C"))
  (`self.K2_CommitAbility`)
  ; EXTENDED weapons manager component
  (`/Engine/EditorBlueprintResources/StandardMacros.IsValid` _returnvalue
    (:`Is Valid`
      (`|ExecutionSequence`
        (:`then_0`
          (`|SwitchGameplayTag` (`|GetArrayItem` (`BlueprintGameplayTagLibrary.BreakGameplayTagContainer` (`.TargetTags` (break `GameplayEventData` EventData))))
            (:`Default`
              (`/Game/_DEV/Weapons/WeaponsManagerComponent.UnequipWeapon` _returnvalue))
            (:`Weapon.Ranged.Staff`
              (`/Game/_DEV/Weapons/WeaponsManagerComponent.EquipWeapon` _returnvalue "/Game/_DEV/Weapons/BP_Weapon_Staff.BP_Weapon_Staff_C")
              (`GameplayStatics.PlaySoundAtLocation` "/Game/Assets/Sounds/Creatures/Troll/Sounds/SoundWaves/Grux_Ability_LMB_Engage_010.Grux_Ability_LMB_Engage_010" (0.0 0.0 0.0) (struct) 1.0 1.0 0.0 null null null null))
            (:`Weapon.Melee.Axe`
              (`/Game/_DEV/Weapons/WeaponsManagerComponent.EquipWeapon` _returnvalue "/Game/_DEV/Weapons/BP_Weapon_Axe.BP_Weapon_Axe_C"))
            (:`Weapon.Melee.Shield`
              (`/Game/_DEV/Weapons/WeaponsManagerComponent.EquipWeapon` _returnvalue "/Game/_DEV/Weapons/BP_Weapon_Shield.BP_Weapon_Shield_C"))))
        (:`then_1`
          (`self.K2_EndAbility`))))))