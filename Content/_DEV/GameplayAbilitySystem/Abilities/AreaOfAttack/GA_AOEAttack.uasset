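; Gameplay ability for a targeted area-of-effect attack, aimed with a ground-trace decal during a looping casting montage.
; On confirmation it commits, plays the ground-cast montage with indicator and attack cues, and waits for a montage trigger event.
; After a short delay, the authority sphere-traces pawns, excluding the caster, calling ApplyDamage per hit and applying a SetByCaller damage GameplayEffect once per unique actor.
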(event `self.K2_ActivateAbility`
  (`self.LoopTargetingAnimation`)
  (set `self.IsWaitingTargetData` true)
  (`self.K2_AddGameplayCue` (struct :`TagName` "GameplayCue.TargetingCamera"))
  (bind (_asynctaskproxy _data) (`AbilityTask_WaitTargetData.WaitTargetData` "None" "UserConfirmed" "/Game/_DEV/GameplayAbilitySystem/TargetingActors/GATargetActor_GroundTrace_Decal.GATargetActor_GroundTrace_Decal_C" (* (`self.AOERadius`) 2.0) null 0.0 0.0 999999.0 (struct :`Name` "NoCollision") true (`self.MakeTargetLocationInfoFromOwnerSkeletalMeshComponent` "staff_equipped_socket") (struct) null)
    (:`ValidData`
      (set `self.IsWaitingTargetData` false)
      (set `self.ConfirmedAOELocation` (`.Location` (`GameplayStatics.BreakHitResult` (`AbilitySystemBlueprintLibrary.GetHitResultFromTargetData` _data))))
      (`self.ConfirmStrike`))))

(event `LoopTargetingAnimation`
  (`AbilityTask_PlayMontageAndWait.CreatePlayMontageAndWaitProxy` "None" "/Game/MageAnimationSet/Animations/InPlace/Mage_Telekinesis_Loop_IP_Montage.Mage_Telekinesis_Loop_IP_Montage"
    (:`OnBlendOut`
      (if (`self.IsWaitingTargetData`)
        (`self.LoopTargetingAnimation`)))
    (:`OnInterrupted`
      (if (`self.IsWaitingTargetData`)
        (`self.K2_EndAbility`)))))

(event `ConfirmStrike`
  (bind _returnvalue (`self.K2_CommitAbility`))
  (if _returnvalue
    (`self.K2_AddGameplayCueWithParams` (struct :`TagName` "GameplayCue.AOEIndicator") (`AbilitySystemBlueprintLibrary.MakeGameplayCueParameters` 0.0 (* (`self.AOERadius`) 2.0) (struct) (struct) (struct) (struct) (struct) (`self.ConfirmedAOELocation`) (0.0 0.0 0.0) (`self.GetAvatarActorFromActorInfo`)))
    (`AbilityTask_PlayMontageAndWait.CreatePlayMontageAndWaitProxy` "None" "/Game/CasterAnimationPack/Animations/Casting/A_GroundCast_Montage.A_GroundCast_Montage"
      (:`then`
        (`self.K2_AddGameplayCueWithParams` (struct :`TagName` "GameplayCue.AOEAttack") (`AbilitySystemBlueprintLibrary.MakeGameplayCueParameters` 0.0 (`self.AOERadius`) (struct) (struct) (struct) (struct) (struct) (`self.ConfirmedAOELocation`)))
        (`AbilityTask_WaitGameplayEvent.WaitGameplayEvent` (struct :`TagName` "Event.Montage.Trigger") null
          (:`EventReceived`
            (`KismetSystemLibrary.Delay` 0.2)
            (`self.AOEDamage`)
            (`self.K2_RemoveGameplayCue` (struct :`TagName` "GameplayCue.AOEIndicator")))))
      (:`OnCompleted`
        (`self.K2_EndAbility` :!label _label))
      (:`OnInterrupted`
        (goto _label)))
    (else
      (`self.K2_EndAbility`))))

(event `AOEDamage`
  (bind _confirmedaoelocation (`self.ConfirmedAOELocation`))
  (`self.K2_HasAuthority`
    (:`True`
      (bind _outhits (`KismetSystemLibrary.SphereTraceMultiForObjects` _confirmedaoelocation _confirmedaoelocation (`self.AOERadius`) (`|MakeArray` "ObjectTypeQuery3" :!type "EObjectTypeQuery Enum") false (`|MakeArray` (`self.GetAvatarActorFromActorInfo`))))
      (`KismetArrayLibrary.Array_Clear` (`self.HitActors`))
      (for _array_element _outhits
        (bind (_bblockinghit _binitialoverlap _time _distance _location _impactpoint _normal _impactnormal _physmat _hitactor) (`GameplayStatics.BreakHitResult` _array_element))
        (`GameplayStatics.ApplyDamage` _hitactor (`self.DamageMagnitude`) null null "/Script/Engine.DamageType")
        (if (not (`KismetArrayLibrary.Array_Contains` (`self.HitActors`) _hitactor))
          (`KismetArrayLibrary.Array_AddUnique` (`self.HitActors`) _hitactor)
          (bind _returnvalue (`AbilitySystemBlueprintLibrary.GetAbilitySystemComponent` _hitactor))
          (`/Engine/EditorBlueprintResources/StandardMacros.IsValid` _returnvalue
            (:`Is Valid`
              (bind _returnvalue_2 (`AbilitySystemBlueprintLibrary.AssignTagSetByCallerMagnitude` (`self.MakeOutgoingGameplayEffectSpec` "/Game/_DEV/GameplayAbilitySystem/Effects/GE_Damage_Instant.GE_Damage_Instant_C") (struct :`TagName` "Data.Damage") (`self.DamageMagnitude`)))
              (`AbilitySystemComponent.BP_ApplyGameplayEffectSpecToSelf` _returnvalue _returnvalue_2))))))))